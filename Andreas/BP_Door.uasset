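; Door actor that continuously swings away from or toward either side based on where the player stands, with no range check.
; Each tick, a dot product of the DoorDirection forward vector and the normalized direction to the player decides front or behind.
; The Door component eases toward opposite 90-degree rotations by lerping from its current rotation with delta time as alpha, while debug text prints the detected side.
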(event EventBeginPlay)

(event EventTick
  (params (DeltaSeconds :type Float%20%28single-precision%29))
  (bind _returnvalue (Utilities|Time|GetWorldDeltaSeconds))
  (bind _returnvalue_2 (Game|GetPlayerCharacter 0))
  (bind _door (Variables|Default|GetDoor))
  (bind _door_2 (Variables|Default|GetDoor))
  (Utilities|IsValid _returnvalue_2
    (:Is%20Valid
      (if (> (Math|Vector|DotProduct (Math|Vector|GetForwardVector (Variables|Default|GetDoorDirection)) (Math|Vector|Normalize (- (Transformation|GetActorLocation _returnvalue_2) (Transformation|GetActorLocation)))) 0.0)
        (Development|PrintString "Player is in front!" true true "(R=0.128440,G=1.000000,B=0.000000,A=1.000000)" _returnvalue)
        (Transformation|SetRelativeRotation _door_2 (Math|Rotator|Lerp(Rotator) (Variables|/Script/Engine.SceneComponent|GetRelativeRotation _door_2) "0,-90.000000, 0" (Utilities|Time|GetWorldDeltaSeconds)) false false)
        (else
          (Development|PrintString "Player is behind!" true true "(R=1.000000,G=0.000000,B=0.059606,A=1.000000)" _returnvalue)
          (Transformation|SetRelativeRotation _door (Math|Rotator|Lerp(Rotator) (Variables|/Script/Engine.SceneComponent|GetRelativeRotation _door) "0,90.000000, 0" (Utilities|Time|GetWorldDeltaSeconds)) false false))))))

(fn ConstructionScript)