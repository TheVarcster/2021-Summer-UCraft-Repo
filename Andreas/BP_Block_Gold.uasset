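; Gold block Blueprint, a child of a hittable block class, that completes the player's mission once its hits run out.
; Its HitME override decrements NumberHits while it is above zero, without calling the parent logic.
; A hit at zero casts player 0's character to ThirdPersonCharacter, sets CompletedMission, then runs the parent HitME; a failed cast skips both.
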(event EventBeginPlay
  (|CallParentFunction) ; This node is disabled and will not be called.\nDrag off pins to build functionality.
)

(event Collision|EventActorBeginOverlap
  (params (OtherActor :type Actor%20Object%20Reference))
  (|CallParentFunction OtherActor) ; This node is disabled and will not be called.\nDrag off pins to build functionality.
)

(event EventTick
  (params (DeltaSeconds :type Float%20%28single-precision%29))
  (|CallParentFunction DeltaSeconds) ; This node is disabled and will not be called.\nDrag off pins to build functionality.
)

(event EventParentHitME
  (if (> (Variables|Default|GetNumberHits) 0)
    (Math|Integer|DecrementInt (Variables|Default|GetNumberHits))
    (else
      (bind _asthird_person_character (Utilities|Casting|CastToThirdPersonCharacter (Game|GetPlayerCharacter 0)))
      (Variables|/Game/ThirdPersonBP/Blueprints/ThirdPersonCharacter.ThirdPersonCharacter_C|SetCompletedMission _asthird_person_character true)
      (|CallParentFunction))))

(fn ConstructionScript
  (|CallParentFunction))