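; BP_Cart is an actor that shuttles back and forth between a StartingPoint and an EndPoint actor, starting on BeginPlay.
; The Rails timeline lerps its location between them, with a FlipFlop alternating forward and reverse playback.
; Each finish waits four seconds, then calls ChooChoo again to loop the trip.
; A Levitation timeline for vertical offset exists but is never triggered.
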(event Custom|ChooChoo
  (Utilities|FlowControl|FlipFlop
    (:A
      (bind _motionpath (Timeline|Rails PlayFromStart)
        (:Update
          (Transformation|SetActorLocation (Math|Vector|Lerp(Vector) (Transformation|GetActorLocation (Variables|ANDY|GetStartingPoint)) (Transformation|GetActorLocation (Variables|ANDY|GetEndPoint)) _motionpath) false false))
        (:Finished
          (Utilities|FlowControl|Delay 4.0)
          (CallFunction|ChooChoo))))
    (:B
      (Timeline|Rails ReverseFromEnd))))

(event EventBeginPlay
  (CallFunction|ChooChoo))

(event Collision|EventActorBeginOverlap
  (params (OtherActor :type Actor%20Object%20Reference)))

(event EventTick
  (params (DeltaSeconds :type Float%20%28single-precision%29)))

(fn ConstructionScript)