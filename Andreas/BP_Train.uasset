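; Train actor that shuttles back and forth between a StartingPoint and an EndPoint actor.
; The RailTrack timeline lerps its location between the two points, and a FlipFlop in ChooChoo alternates forward and reverse playback, re-triggered after a pause whenever the timeline finishes.
; A separate Levitation timeline, started on BeginPlay, applies vertical world offsets to the train.
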(event Custom|ChooChoo
  (Utilities|FlowControl|FlipFlop
    (:A
      (bind _motion (Timeline|RailTrack PlayFromStart)
        (:Update
          (Transformation|SetActorLocation (Math|Vector|Lerp(Vector) (Transformation|GetActorLocation (Variables|andy|GetStartingPoint)) (Transformation|GetActorLocation (Variables|andy|GetEndPoint)) _motion) false false))
        (:Finished
          (Utilities|FlowControl|Delay 5.0)
          (CallFunction|ChooChoo))))
    (:B
      (Timeline|RailTrack ReverseFromEnd))))

(event EventBeginPlay
  (CallFunction|ChooChoo)
  (bind _motion (Timeline|Levitation PlayFromStart)
    (:Update
      (Transformation|AddActorWorldOffset (Math|Vector|MakeVector 0.0 0.0 _motion)))))

(fn ConstructionScript)