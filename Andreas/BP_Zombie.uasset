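; BP_Zombie is a zombie pawn Blueprint that wanders the map and can chase the player.
; From BeginPlay, WanderAroud repeatedly uses AI MoveTo toward a random reachable point nearby, pausing briefly after success or failure before calling itself again.
; A separate CHASE event moves it to the first player's character, but nothing in this file calls it or stops the wander loop.
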(event Custom|CHASE
  (AI|AIMoveTo self "0, 0, 0" (Game|GetPlayerCharacter 0) 5.0 false))

(event Custom|WanderAroud
  (AI|AIMoveTo self (.RandomLocation (AI|Navigation|GetRandomReachablePointinRadius (Transformation|GetActorLocation) 7.2e+02 0 0)) 0 5.0 false
    (:OnSuccess
      _)
    (:OnFail
      _))
  (Utilities|FlowControl|Delay 2.0)
  (CallFunction|WanderAroud))

(event EventBeginPlay
  (CallFunction|WanderAroud))

(event Collision|EventActorBeginOverlap
  (params (OtherActor :type Actor%20Object%20Reference)))

(event EventTick
  (params (DeltaSeconds :type Float%20%28single-precision%29)))

(fn ConstructionScript)