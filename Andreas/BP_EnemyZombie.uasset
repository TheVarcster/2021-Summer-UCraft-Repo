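; BP_EnemyZombie is an enemy zombie Blueprint that wanders at random and can charge the player.
; From BeginPlay, WanderAround uses AI MoveTo toward a random reachable point near its current location, then calls itself after a short delay on success or failure.
; A separate ChargePlayer event moves it toward the player character, but nothing in this graph calls that event.
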(event Custom|WanderAround
  (AI|AIMoveTo self (.RandomLocation (AI|Navigation|GetRandomReachablePointinRadius (Transformation|GetActorLocation) 999.0 0 0)) 0 5.0 false
    (:OnSuccess
      _)
    (:OnFail
      _))
  (Utilities|FlowControl|Delay 2.0)
  (CallFunction|WanderAround))

(event Custom|ChargePlayer
  (AI|AIMoveTo self "0, 0, 0" (Game|GetPlayerCharacter 0) 5.0 false))

(event EventBeginPlay
  (CallFunction|WanderAround))

(event Collision|EventActorBeginOverlap
  (params (OtherActor :type Actor%20Object%20Reference)))

(event EventTick
  (params (DeltaSeconds :type Float%20%28single-precision%29)))

(fn ConstructionScript)